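; BP_ImpactEffects is an impact effects actor that plays a particle, sound and decal at a hit point on BeginPlay.
; It first builds a decal rotation from the HitResult normal's roll and pitch with a random yaw.
; It then switches on the physical material's surface type, though only default assets appear, and attaches a sized, timed decal to the hit component.
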(event EventBeginPlay
  (bind _hitresult (Variables|Default|GetHitResult))
  (bind _hitresult_2 (Variables|Default|GetHitResult))
  (bind _decalsize (Variables|Default|GetDecalSize))
  (bind _normal (Collision|BreakHitResult _hitresult))
  (bind (_bblockinghit _binitialoverlap _time _location _impactpoint _normal_2 _impactnormal _physmat _hitactor _hitcomponent) (Collision|BreakHitResult _hitresult_2))
  (bind _returnvalue (Math|Conversions|RotationFromXVector _normal))
  (bind (_roll _pitch) (Math|Rotator|BreakRotator _returnvalue))
  (Utilities|FlowControl|Sequence
    (:then_0
      (Variables|Default|SetRandomDecalRotation (Math|Rotator|MakeRotator _roll _pitch (Math|Random|RandomFloatinRange -1.8e+02 1.8e+02))))
    (:then_1
      (switch Utilities|FlowControl|Switch|SwitchonEPhysicalSurface (Variables|/Script/Engine.PhysicalMaterial|GetSurfaceType _physmat)
        (:SurfaceType_Default
          (Effects|SpawnEmitteratLocation (Variables|Default|GetDefaultFX) _impactpoint)
          (Audio|PlaySoundatLocation (Variables|Default|GetDefaultSound) _impactpoint)
          (Class|GameplayStatics|SpawnDecalAttached (Variables|Default|GetDefaultDecalMat) (Math|Vector|MakeVector _decalsize _decalsize 1.0) _hitcomponent "None" _impactpoint (Variables|Default|GetRandomDecalRotation) "KeepRelativeOffset" (Variables|Default|GetDecalLifeSpan)))))))

(event EventActorBeginOverlap
  (params (OtherActor :type Actor%20Object%20Reference)))

(event EventTick
  (params (DeltaSeconds :type Float%20%28single-precision%29)))

(fn ConstructionScript)